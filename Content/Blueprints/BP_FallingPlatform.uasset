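; A platform that drops shortly after the third-person character steps on it, then returns to its starting spot.
; A box trigger overlap starts the cycle if the platform is ready: countdown delay, physics-simulated fall, then reset.
; Reset disables physics and uses a timeline to lerp from the fallen transform to the one saved at BeginPlay, then re-arms.
; Each phase swaps the material and prints a debug message.
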(event OnComponentBeginOverlap(BoxTrigger)
  (params (OverlappedComponent :type Primitive%20Component%20Object%20Reference) (OtherActor :type Actor%20Object%20Reference) (OtherComp :type Primitive%20Component%20Object%20Reference) (OtherBodyIndex :type Integer) (bFromSweep :type Boolean) (SweepResult :type Hit%20Result%20Structure%20%28by%20ref%29))
  ;[0.15 0.15 0.15 0.5] Comment
  (Development|PrintString "Something is standing on me")
  (if (Variables|Default|GetisReady) ; is the platform ready?
    (Utilities|Casting|CastToBP_ThirdPersonCharacter OtherActor)
    (CallFunction|Activate)))

(event Custom|Activate
  (Variables|Default|SetisReady false) ; we're working, we cannot\nbe activated until we're reset
  (Development|PrintString "Starting Countdown!")
  (Rendering|Material|SetMaterial (Variables|Default|GetPlatform) 0 "/Game/Materials/FallingPlatforms/MI_ActivePlatform.MI_ActivePlatform")
  (Utilities|FlowControl|Delay (Variables|PlatformSettings|GetFallDelayDuration)) ; wait a second
  (CallFunction|Fall))

(event Custom|Fall
  (Development|PrintString "Falling!")
  (Rendering|Material|SetMaterial (Variables|Default|GetPlatform) 0 "/Game/Materials/FallingPlatforms/MI_FallingPlatform.MI_FallingPlatform")
  (Physics|SetSimulatePhysics (Variables|Default|GetPlatform) true) ; This allows the platform to be affected \nby physics (gravity, for example)
  (Utilities|FlowControl|Delay (Variables|PlatformSettings|GetFall%20Duration)) ; wait 3 seconds
  (CallFunction|Reset))

(event Custom|Reset
  (Development|PrintString "Resetting the platform")
  (Rendering|Material|SetMaterial (Variables|Default|GetPlatform) 0 "/Game/Materials/FallingPlatforms/MI_ResettingPlatform.MI_ResettingPlatform")
  (Physics|SetSimulatePhysics (Variables|Default|GetPlatform) false) ; This stops the platform from being affected \nby physics (gravity, for example)
  (Variables|Default|SetFallenTransform (Transformation|GetWorldTransform (Variables|Default|GetPlatform))) ; capture the position of the platform\nright before we start resetting it
  (bind _newtrack_0 (Timeline|GoBackToStartTransform PlayFromStart)
    (:Update
      ;[0.15 0.15 0.15 0.5] Timeline update
      (Transformation|SetWorldTransform (Variables|Default|GetPlatform) (Math|Transform|Lerp(Transform) (Variables|Default|GetFallenTransform) (Variables|Default|GetStartingTransform) _newtrack_0) false false))
    (:Finished
      ;[0.15 0.15 0.15 0.5] timeline finished
      (Variables|Default|SetisReady true) ; we've been reset, \nwalk on us again plz
      (Rendering|Material|SetMaterial (Variables|Default|GetPlatform) 0 "/Game/Materials/FallingPlatforms/MI_ReadyPlatform.MI_ReadyPlatform"))))

(event EventBeginPlay
  ;[0.15 0.15 0.15 0.5] Comment
  (Variables|Default|SetStartingTransform (Transformation|GetWorldTransform (Variables|Default|GetPlatform))) ; capture the starting position and rotation\nof the platform.
)

(fn ConstructionScript)